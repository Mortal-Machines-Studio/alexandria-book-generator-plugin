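; Custom PCG node that generates a row of points for books, each tagged with a BookMesh attribute on the Points output.
; Picks seeded random meshes from the Meshes input's soft-path attribute, then blocking-loads each to read width and pivot offset.
; Spaces books along the owner's local X axis by stack direction with random gaps, converting to world space with position-derived point seeds.
; PointLoop then sets point extents and writes the stored mesh paths.
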(fn NodeTitleOverride
  (return "Generate Points For Books"))

(fn ExecutewithContext
  (params (InContext :type PCG%20Context%20Structure%20%28by%20ref%29) (Input :type PCG%20Data%20Collection%20Structure%20%28by%20ref%29))
  (Variables|Default|SetGraphInputs Input)
  (Utilities|FlowControl|Sequence
    (:then_0
      (Variables|Default|SetSeed (Class|PCGBlueprintElement|GetSeed InContext))
      (Math|Random|SetRandomStreamSeed (Variables|Default|GetStreamSeed) (Variables|Default|GetSeed)))
    (:then_1
      (bind _returnvalue (Game|ConstructObjectfromClass "/Script/PCG.PCGPointData"))
      (bind _output_get (LocalVariables|SetPointData _returnvalue))
      (bind _returnvalue_2 (Metadata|MutableMetadata _output_get))
      (LocalVariables|SetOutMetadata _returnvalue_2)
      (Generation|GeneratePoints)
      (SpatialData|SetPoints (LocalVariables|GetPointData) (Variables|Default|GetPointsToCreate))
      (PCG|Metadata|CreateSoftObjectPathAttribute (LocalVariables|GetOutMetadata) "BookMesh" (Book|GetRandomBookMesh Input) false true)
      (bind _outdata (PCG|FlowControl|PointLoop InContext (LocalVariables|GetPointData) 0))
      (return (Utilities|Struct|MakePCGDataCollection (Utilities|Array|MakeArray (Utilities|Struct|MakePCGTaggedData _outdata 0 "Points")))))))

(fn PointLoopBody
  (params (InContext :type PCG%20Context%20Structure%20%28by%20ref%29) (InData :type PCG%20Point%20Data%20Object%20Reference) (InPoint :type PCG%20Point%20Structure%20%28by%20ref%29) (OutMetadata :type PCG%20Metadata%20Object%20Reference) (Iteration :type Integer64))
  (Class|PCGBlueprintHelpers|SetExtents InPoint (Math|Vector|MakeVector 1.0 1.0 1.0))
  (LocalVariables|SetBookMeshSoftObjectPath (Book|GetRandomBookMesh (Variables|Default|GetGraphInputs)))
  (Class|PCGMetadataAccessorHelpers|SetSoftObjectPathAttribute InPoint OutMetadata "BookMesh" (Utilities|Array|Get(acopy) (Variables|Default|GetGeneratedBooksMeshes) (Math|Conversions|ToInteger(Byte) Iteration)))
  (return InPoint true))

(fn GetRandomBookMesh
  (params (Inputs :type PCG%20Data%20Collection%20Structure%20%28by%20ref%29))
  (bind _returnvalue (Data|GetInputsbyPinLabel Inputs "Meshes"))
  (for _array_element _returnvalue
    (bind _aspcgattribute_set (Utilities|Casting|CastToPCGParamData (.Data (Utilities|Struct|BreakPCGTaggedData _array_element))))
    (bind _returnvalue_2 (Metadata|MutableMetadata _aspcgattribute_set))
    (bind _output_get (LocalVariables|SetInMetadata _returnvalue_2))
    (LocalVariables|SetNumberOfMeshes (Math|Conversions|ToInteger(Byte) (Class|PCGMetadata|GetItemCountforChild _output_get)))
    (LocalVariables|SetMeshAttributeName (Utilities|Array|Get(acopy) (.AttributeNames (PCG|Metadata|GetAttributes _output_get)) (Utilities|Array|LastIndex (.AttributeNames (PCG|Metadata|GetAttributes _output_get)))))
    (switch Utilities|FlowControl|Switch|SwitchonEPCGMetadataTypes (Utilities|Array|Get(acopy) (.AttributeTypes (PCG|Metadata|GetAttributes _output_get)) (Utilities|Array|LastIndex (.AttributeNames (PCG|Metadata|GetAttributes _output_get))))
      (:SoftObjectPath
        (bind _returnvalue_3 (PCG|Metadata|GetSoftObjectPathAttributebyMetadataKey (Class|KismetMathLibrary|ToInt64(Integer) (Class|KismetMathLibrary|RandomIntegerfromStream (Variables|Default|GetStreamSeed) (LocalVariables|GetNumberOfMeshes))) (LocalVariables|GetInMetadata) (LocalVariables|GetMeshAttributeName)))
        (return _returnvalue_3)))))

(fn GeneratePoints
  (bind _gaprange (Variables|Default|GetGapRange))
  (LocalVariables|SetOwnerTransform (Getters|GetOwnerTransform))
  (for _index (range 0 (- (Variables|Default|GetNumBooks) 1))
    (LocalVariables|SetCurrentIndex _index)
    (bind _output_get (LocalVariables|SetNewBookMesh (Book|GetRandomBookMesh (Variables|Default|GetGraphInputs))))
    (Utilities|Array|Add (Variables|Default|GetGeneratedBooksMeshes) _output_get)
    (Utilities|FlowControl|Sequence
      (:then_0
        (bind (_location _pivotoffset) (Book|GetBookPosition (LocalVariables|GetNewBookMesh) (LocalVariables|GetCurrentIndex)))
        (Variables|Default|SetCurrentBookLocation _location)
        (LocalVariables|SetPivotOffset _pivotoffset))
      (:then_1
        (bind _output_get_2 (LocalVariables|SetWorldSpaceTransform (Helpers|ConvertPointtoWorldSpace (Variables|Default|GetCurrentBookLocation) (LocalVariables|GetOwnerTransform))))
        (bind _returnvalue (PCG|Helpers|ComputeSeedfromPosition (.Location (Math|Transform|BreakTransform _output_get_2))))
        (LocalVariables|SetPointSeed _returnvalue)
        (Utilities|Array|Add (Variables|Default|GetPointsToCreate) (Utilities|Struct|MakePCGPoint (Math|Transform|MakeTransform (.Location (Math|Transform|BreakTransform _output_get_2)) (.Rotation (Math|Transform|BreakTransform _output_get_2)) "1.000000,1.000000,1.000000") 1.0 "-1.000000,-1.000000,-1.000000" "1.000000,1.000000,1.000000" "(X=1.000000,Y=1.000000,Z=1.000000,W=1.000000)" 0.5 (LocalVariables|GetPointSeed)))
        (Variables|Default|SetCurrentBookLocation (Utilities|Select :Index (Variables|Default|GetStackDirection) :NewEnumerator0 (+ (Variables|Default|GetCurrentBookLocation) (Math|Vector|MakeVector (+ (LocalVariables|GetPivotOffset) (Math|Random|RandomFloatinRangefromStream (Variables|Default|GetStreamSeed) (.x _gaprange) (.y _gaprange))) 0.0 0.0)) :NewEnumerator1 (- (Variables|Default|GetCurrentBookLocation) (Math|Vector|MakeVector (+ (LocalVariables|GetPivotOffset) (Math|Random|RandomFloatinRangefromStream (Variables|Default|GetStreamSeed) (.x _gaprange) (.y _gaprange))) 0.0 0.0)))))))
  (return))

(fn GetBookPosition
  (params (BookMesh :type Soft%20Object%20Path%20Structure) (Index :type Integer))
  (bind _returnvalue (Utilities|LoadAssetBlocking (Class|KismetSystemLibrary|ToSoftObjRef(SoftObjPath) BookMesh)))
  (bind _asstatic_mesh (Utilities|Casting|CastToStaticMesh _returnvalue))
  (bind _output_get (LocalVariables|SetBookStaticMesh _asstatic_mesh))
  (Utilities|IsValid _output_get
    (:Is%20Valid
      (switch Utilities|FlowControl|Switch|SwitchonE_BookStackDirection (Variables|Default|GetStackDirection)
        (:NewEnumerator0
          (return (Math|Vector|MakeVector (+ (.x (Variables|Default|GetCurrentBookLocation)) (- (Book|GetBookWidth (LocalVariables|GetBookStaticMesh)) (* (Book|GetMeshPivotOffset (LocalVariables|GetBookStaticMesh)) -1.0))) 0.0 0.0) (* (Book|GetMeshPivotOffset (LocalVariables|GetBookStaticMesh)) -1.0)))
        (:NewEnumerator1
          (return (Math|Vector|MakeVector (Math|Float|SelectFloat (- (.x (Variables|Default|GetCurrentBookLocation)) (* (Book|GetMeshPivotOffset (LocalVariables|GetBookStaticMesh)) -1.0)) 0.0 (> Index 0)) 0.0 0.0) (- (Book|GetBookWidth (LocalVariables|GetBookStaticMesh)) (* (Book|GetMeshPivotOffset (LocalVariables|GetBookStaticMesh)) -1.0))))))))

(fn GetBookWidth
  (params (BookMesh :type Static%20Mesh%20Object%20Reference))
  (Utilities|IsValid BookMesh
    (:Is%20Valid
      (return (Math|Float|Absolute(Float) (* (.X (Math|Vector|BreakVector (.BoxExtent (Math|BoxSphereBounds|BreakBoxSphereBounds (StaticMesh|GetBounds BookMesh))))) 2.0))))
    (:Is%20Not%20Valid
      (return 0.0))))

(fn GetMeshPivotOffset
  (params (BookMesh :type Static%20Mesh%20Object%20Reference))
  (Utilities|IsValid BookMesh
    (:Is%20Valid
      (return (.X (Math|Vector|BreakVector (.Min (Utilities|Struct|BreakBox (StaticMesh|GetBoundingBox BookMesh)))))))
    (:Is%20Not%20Valid
      (return 0.0))))

(fn GetOwnerTransform
  (bind _returnvalue (PCG|Temporary|GetOriginalComponent (SoundLibrary|GetContext)))
  (return (Math|Transform|MakeTransform (.location (Transformation|GetActorTransform (Components|GetOwner _returnvalue))) (.rotation (Transformation|GetActorTransform (Components|GetOwner _returnvalue))) "1.000000,1.000000,1.000000")))

(fn ConvertPointtoWorldSpace
  (params (PointLocation :type Vector) (OwnerTransform :type Transform))
  (return (Math|Transform|MakeTransform (Math|Transform|TransformLocation OwnerTransform PointLocation) (Math|Transform|TransformRotation OwnerTransform (Utilities|Select :Index (Variables|Default|GetStackDirection) :NewEnumerator0 "0.000000,180.000000,0.000000" :NewEnumerator1 "0.000000,180.000000,0.000000")) "1.000000,1.000000,1.000000")))

(fn GetBookHeight
  (params (BookMesh :type Static%20Mesh%20Object%20Reference))
  (Utilities|IsValid BookMesh
    (:Is%20Valid
      (return (Math|Float|Absolute(Float) (* (.Z (Math|Vector|BreakVector (.BoxExtent (Math|BoxSphereBounds|BreakBoxSphereBounds (StaticMesh|GetBounds BookMesh))))) 2.0))))
    (:Is%20Not%20Valid
      (return 0.0))))